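; BookshelfBP is a secret bookshelf door with a special book, toggled by an Open/Close event.
; A DoOnce, reset when each timeline finishes, blocks retriggering while a FlipFlop alternates between two timelines.
; The first rolls the book between in and out angles while holding the bookshelf's yaw at the closed value.
; The second plays in reverse, but its yaw Lerp runs zero to zero, so the shelf never swings as wired.
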(event `Open/Close`
  (`/Engine/EditorBlueprintResources/StandardMacros.DoOnce` false :!label _label
    (:`Completed`
      (`/Engine/EditorBlueprintResources/StandardMacros.FlipFlop`
        (:`A`
          (bind (_direction _newtrack_0) (`Timeline|Timeline_0` :!via `PlayFromStart`)
            (:`Update`
              (`SceneComponent.K2_SetRelativeRotation` (`self.SpecialBook`) (`KismetMathLibrary.MakeRotator` (`KismetMathLibrary.Lerp` (`self.Bookin`) (`self.Bookout`) _newtrack_0)) false false)
              (`SceneComponent.K2_SetRelativeRotation` (`self.Bookshelf`) (`KismetMathLibrary.MakeRotator` 0.0 0.0 (`KismetMathLibrary.Lerp` (`self.Doorclosed`) (`self.Dooropen`))) false false))
            (:`Finished`
              (goto _label :!via `Reset`))))
        (:`B`
          (bind (_direction_2 _newtrack_0_2) (`Timeline|Timeline_1` :!via `ReverseFromEnd`)
            (:`Update`
              (`SceneComponent.K2_SetRelativeRotation` (`self.Bookshelf`) (`KismetMathLibrary.MakeRotator` 0.0 0.0 (`KismetMathLibrary.Lerp` 0.0 0.0 _newtrack_0_2)) false false))
            (:`Finished`
              (goto _label :!via `Reset`))))))))

(fn `UserConstructionScript`)